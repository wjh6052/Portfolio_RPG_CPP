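; BP_EndBossSkill is an animation notify that marks the end of a boss skill.
; It casts the mesh owner to CCharacter_Boss and writes the current skill's cooldown into the boss's cooldown array at the current index.
; It then clears the OnSkill flag and sets the stat component's speed back to jogging.
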(fn ReceivedNotify
  (params (MeshComp :type Skeletal%20Mesh%20Component%20Object%20Reference) (Animation :type Anim%20Sequence%20Base%20Object%20Reference) (EventReference :type Anim%20Notify%20Event%20Reference%20Structure%20%28by%20ref%29))
  (bind _asccharacter_boss (Utilities|Casting|CastToCCharacter_Boss (Components|GetOwner MeshComp)))
  (Utilities|Array|SetArrayElem (Variables|/Script/Portfolio_RPG_CPP.CCharacter_Boss|GetCurrentSkillCooldownArr _asccharacter_boss) (Variables|/Script/Portfolio_RPG_CPP.CCharacter_Boss|GetCurrentIndex _asccharacter_boss) (Utilities|Struct|BreakSkill (Variables|/Script/Portfolio_RPG_CPP.CCharacter_Boss|GetCurrentSkill _asccharacter_boss)))
  (Variables|/Script/Portfolio_RPG_CPP.CCharacter_Boss|SetbOnSkill _asccharacter_boss false)
  (Class|CStatComponent|SetSpeed (Class|CCharacterBase|GetStatComponent _asccharacter_boss) "Joging")
  (return false))